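; BP_NodePortal is a see-through portal actor that pairs with a TargetPortal to show a live view between the two.
; At BeginPlay its scene capture renders to a viewport-sized render target, displayed on the target's mesh through a dynamic M_NodePortal material.
; Each Tick drives the target's capture from the player's portal-relative position and quaternion-composed camera rotation, with a clip plane enabled along the target mesh's forward vector.
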(event EventBeginPlay
  (bind _returnvalue (Viewport|GetViewportSize))
  (Utilities|FlowControl|Sequence
    (:then_0
      (Utilities|IsValid (Variables|Default|GetTarget%20%20Portal)
        (:Is%20Valid
          (if true
            (bind _returnvalue_2 (Rendering|CreateRenderTarget2D (Math|Float|Truncate (.x _returnvalue)) (Math|Float|Truncate (.y _returnvalue)) "RTF_RGBA16f"))
            (bind _output_get (Variables|/Script/Engine.SceneCaptureComponent2D|SetTextureTarget (Variables|Default|GetSceneCaptureComponent2D) _returnvalue_2))
            (bind _returnvalue_3 (Rendering|Material|CreateDynamicMaterialInstance "/Game/Node_Portals/M_NodePortal.M_NodePortal" "None" :!class /Script/Engine.KismetMaterialLibrary))
            (Rendering|Material|SetTextureParameterValue _returnvalue_3 "Portal Texture" _output_get)
            (bind _newparam (CallFunction|GetMesh (Variables|Default|GetTarget%20%20Portal)))
            (Rendering|Material|SetMaterial _newparam 0 _returnvalue_3)))))
    (:then_1
      (Variables|Default|SetPlayer (Game|Player|GetPlayerPawn 0)))))

(event EventTick
  (params (DeltaSeconds :type Float%20%28single-precision%29))
  (bind _returnvalue (Game|GetPlayerCameraManager 0))
  (bind _returnvalue_2 (Transformation|GetActorTransform))
  (bind _returnvalue_3 (Transformation|GetActorRotation))
  (bind _target__portal (Variables|Default|GetTarget%20%20Portal))
  (bind _target__portal_2 (Variables|Default|GetTarget%20%20Portal))
  (bind _target__portal_3 (Variables|Default|GetTarget%20%20Portal))
  (bind _player (Variables|Default|GetPlayer))
  (bind _staticmeshcomponent (Variables|Debug|GetStaticMeshComponent))
  (bind _staticmeshcomponent_2 (Variables|Debug|GetStaticMeshComponent))
  (bind _returnvalue_4 (Transformation|GetWorldLocation _staticmeshcomponent_2))
  (bind _returnvalue_5 (Camera|GetCameraRotation _returnvalue))
  (bind _returnvalue_6 (Math|Transform|InverseTransformRotation _returnvalue_2 _returnvalue_3))
  (bind _returnvalue_7 (Transformation|GetActorRotation _target__portal_3))
  (bind _returnvalue_8 (Transformation|GetActorTransform _target__portal_3))
  (bind _returnvalue_9 (Transformation|GetActorLocation _player))
  (bind (_roll _pitch _yaw) (Math|Rotator|BreakRotator _returnvalue_5))
  (bind (_roll_2 _pitch_2 _yaw_2) (Math|Rotator|BreakRotator _returnvalue_6))
  (bind _returnvalue_10 (Math|Transform|TransformRotation _returnvalue_8 _returnvalue_7))
  (bind _returnvalue_11 (- _returnvalue_9 _returnvalue_4))
  (bind (_roll_3 _pitch_3 _yaw_3) (Math|Rotator|BreakRotator _returnvalue_10))
  (Utilities|IsValid _target__portal
    (:Is%20Valid
      (bind _scene_capture (CallFunction|GetSceneCapture _target__portal))
      (bind _newparam (CallFunction|GetMesh _target__portal_2))
      (Variables|/Script/Engine.SceneCaptureComponent2D|SetbEnableClipPlane _scene_capture true)
      (bind _output_get (Variables|/Script/Engine.SceneCaptureComponent2D|SetClipPlaneNormal _scene_capture (Math|Vector|GetForwardVector _newparam)))
      (Variables|/Script/Engine.SceneCaptureComponent2D|SetClipPlaneBase _scene_capture (+ _output_get (Math|Vector|GetForwardVector _newparam)))
      (Transformation|SetWorldLocation _scene_capture (+ (* (+ (* (Math|Vector|GetForwardVector _newparam) (Math|Vector|DotProduct _returnvalue_11 (Math|Vector|GetForwardVector _staticmeshcomponent))) (* (Math|Vector|GetRightVector _newparam) (Math|Vector|DotProduct _returnvalue_11 (Math|Vector|GetRightVector _staticmeshcomponent)))) -1.0) (* (Math|Vector|GetUpVector _newparam) (Math|Vector|DotProduct _returnvalue_11 (Math|Vector|GetUpVector _staticmeshcomponent))) (Transformation|GetActorLocation _target__portal_2)) false false)
      (bind _scene_capture_2 (CallFunction|GetSceneCapture _target__portal_3))
      (Transformation|SetWorldRotation _scene_capture_2 (Class|KismetMathLibrary|QuatRotator (* (Class|KismetMathLibrary|ToQuaterion(Vector) (Math|Vector|MakeVector _roll_3 _pitch_3 _yaw_3)) (* (Class|KismetMathLibrary|ToQuaterion(Vector) (Math|Vector|MakeVector _roll_2 _pitch_2 _yaw_2)) (Class|KismetMathLibrary|ToQuaterion(Vector) (Math|Vector|MakeVector _roll _pitch _yaw))))) false false))))

(fn ConstructionScript)

(fn GetSceneCapture
  (return (Variables|Default|GetSceneCaptureComponent2D)))

(fn GetMesh
  (return (Variables|Debug|GetStaticMeshComponent)))